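; BP_Weapon is a weapon Blueprint that breaks and scatters Chaos destructible objects at a given location.
; CreateFields applies a radial-falloff external strain field within a small sphere to fracture clusters, then a radial vector linear velocity field to push pieces away from that point.
; It also draws a short-lived debug sphere at the strain radius.
; BeginPlay, overlap and construction logic are empty, and nothing in this file calls CreateFields.
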(event `self.CreateFields`
  (params (location :type "Vector Structure (by ref)"))
  (set `self.FieldLocation` location)
  (set `self.SphereRadius` 25.0)
  (`FieldSystemComponent.ApplyPhysicsField` (`self.FieldSystem`) true "Field_ExternalClusterStrain" (`self.FieldSystemMetaDataFilter`) (`RadialFalloff.SetRadialFalloff` (`self.RadialFalloff`) 500000.0 0.0 1.0 0.0 (`self.SphereRadius`) (`self.FieldLocation`) "Field_FallOff_None"))
  (`FieldSystemComponent.ApplyPhysicsField` (`self.FieldSystem`) true "Field_LinearVelocity" (`self.FieldSystemMetaDataFilter`) (`RadialVector.SetRadialVector` (`self.RadialVector`) 500.0 (`self.FieldLocation`)))
  (`KismetSystemLibrary.DrawDebugSphere` (`self.FieldLocation`) (`self.SphereRadius`) 12 (struct :`R` 1.0 :`B` 0.060523 :`A` 1.0) 2.0 1.0))

(fn `UserConstructionScript`)