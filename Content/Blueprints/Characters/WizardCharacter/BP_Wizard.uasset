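; BP_Wizard is the wizard character Blueprint, currently serving as an on-screen debug readout of wizard state.
; Every Tick prints the player, action and item states plus colliding item, weapon and held item, using keyed colored PrintString calls.
; Disconnected logic would interpolate the capsule toward controller rotation while aiming or attacking, switching between orient-to-movement and controller yaw.
; BeginPlay, overlap and construction script are empty.
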(event `self.ReceiveBeginPlay`)

(event `self.ReceiveTick`
  (params (DeltaSeconds :type "Float (single-precision)"))
  (set `self.Delta Seconds` DeltaSeconds)
  ;[1 1 1] Print player state
  (bind _returnvalue (`self.GetWizardPState`))
  (`KismetSystemLibrary.PrintString` (`|GetEnumeratorNameAsString` _returnvalue) true false (struct :`G` 0.66 :`B` 1.0 :`A` 1.0) -1.0 "312")
  ;[1 1 1] print player action state
  (bind _returnvalue_2 (`self.GetWizardAState`))
  (`KismetSystemLibrary.PrintString` (`|GetEnumeratorNameAsString` _returnvalue_2) true false (struct :`R` 0.697917 :`G` 0.212886 :`A` 1.0) -1.0 "7689")
  ;[1 1 1] Print player item state
  (bind _returnvalue_3 (`self.GetWizardIState`))
  (`KismetSystemLibrary.PrintString` (`|GetEnumeratorNameAsString` _returnvalue_3) true false (struct :`G` 0.222917 :`B` 0.028767 :`A` 1.0) -1.0 "99")
  ;[1 1 1] print player colliding item
  (bind _returnvalue_4 (`self.GetCollidingItem`))
  (`KismetSystemLibrary.PrintString` (`KismetSystemLibrary.GetObjectName` _returnvalue_4) true false (struct :`R` 0.94902 :`G` 1.0 :`A` 1.0) -1.0 "333")
  ;[1 1 1] print player weapon
  (bind _returnvalue_5 (`self.GetPlayerWeapon`))
  (`KismetSystemLibrary.PrintString` (`KismetSystemLibrary.GetObjectName` _returnvalue_5) true false (struct :`R` 0.126793 :`G` 0.272917 :`B` 0.141552 :`A` 1.0) -1.0 "1199")
  ;[1 1 1] print player item
  (bind _returnvalue_6 (`self.GetPlayerItem`))
  (`KismetSystemLibrary.PrintString` (`KismetSystemLibrary.GetObjectName` _returnvalue_6) true false (struct :`R` 0.729726 :`G` 0.747917 :`B` 0.391098 :`A` 1.0) -1.0 "454"))

(fn `UserConstructionScript`)